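; Well actor that builds itself in the construction script from a spline and a PCG graph, with no runtime logic.
; It tiles spline mesh segments along Z, sized by mesh bounds and actor scale, with tangents clamped to segment length and query-and-probe collision.
; It assigns the PCG graph and writes scale-adjusted Radius and Thickness parameters to that graph asset rather than the component.
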(event EventBeginPlay)

(event Collision|EventActorBeginOverlap
  (params (OtherActor :type Actor%20Object%20Reference)))

(event EventTick
  (params (DeltaSeconds :type Float%20%28single-precision%29)))

(fn ConstructionScript
  (bind _returnvalue (Transformation|GetActorScale3D))
  (bind _returnvalue_2 (Transformation|GetActorScale3D))
  (bind _mesh (Variables|Default|GetMesh))
  (bind _radius (Variables|Default|GetRadius))
  (bind _returnvalue_3 (StaticMesh|GetBoundingBox _mesh))
  (bind _returnvalue_4 (Math|Vector|VectorLength _returnvalue_2))
  (bind _returnvalue_5 (* _returnvalue_4 _radius))
  (Class|PCGComponent|SetGraph (Variables|Default|GetPCG) (Variables|Default|GetPCGGraph))
  (bind _output_get (Variables|Default|SetMeshLength (* (.z (+ (Math|Vector|VectorGetAbs (.min _returnvalue_3)) (Math|Vector|VectorGetAbs (.max _returnvalue_3)))) (Math|Vector|VectorLength (Transformation|GetActorScale3D)))))
  (for _index (range 0 (- (Math|Float|Truncate (/ (Spline|GetSplineLength (Variables|Default|GetSpline)) _output_get)) 1))
    (bind _returnvalue_6 (AddComponent|AddSplineMeshComponent false))
    (bind _output_get_2 (Variables|Default|SetSplineMesh _returnvalue_6))
    (Rendering|Material|SetMaterial (Variables|Default|GetSplineMesh) 0 (Variables|Default|GetSplineMeshMaterial))
    (SplineMesh|SetForwardAxis _output_get_2 "Z" true)
    (Components|StaticMesh|SetStaticMesh (Variables|Default|GetSplineMesh) (Variables|Default|GetMesh))
    (Transformation|SetWorldScale3D (Variables|Default|GetSplineMesh) (Math|Vector|MakeVector (.x _returnvalue) (.y _returnvalue) (.z _returnvalue)))
    (SplineMesh|SetStartandEnd (Variables|Default|GetSplineMesh) (Spline|GetLocationatDistanceAlongSpline (Variables|Default|GetSpline) (* _index (Variables|Default|GetMeshLength)) "Local") (Math|Vector|ClampVectorSize (Spline|GetTangentatDistanceAlongSpline (Variables|Default|GetSpline) (* _index (Variables|Default|GetMeshLength)) "Local") 0.0 (Variables|Default|GetMeshLength)) (Spline|GetLocationatDistanceAlongSpline (Variables|Default|GetSpline) (* (+ _index 1) (Variables|Default|GetMeshLength)) "Local") (Math|Vector|ClampVectorSize (Spline|GetTangentatDistanceAlongSpline (Variables|Default|GetSpline) (* (+ _index 1) (Variables|Default|GetMeshLength)) "Local") 0.0 (Variables|Default|GetMeshLength)) true :!class /Script/Engine.SplineMeshComponent)
    (Collision|SetCollisionEnabled (Variables|Default|GetSplineMesh) "QueryAndProbe"))
  (Effects|Components|ParticleSystem|SetFloatParameter (Variables|Default|GetPCGGraph) "Radius" _returnvalue_5)
  (Effects|Components|ParticleSystem|SetFloatParameter (Variables|Default|GetPCGGraph) "Thickness" (+ _returnvalue_5 (Variables|Default|GetThickness))))